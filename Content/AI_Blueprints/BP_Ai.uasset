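; BP_Ai is an AI pawn that reacts to seeing the first-person player and ragdolls on contact with them.
; PawnSensing sets a Chasing flag, which nothing here reads, and starts an AIMoveTo re-issued on a 0.2-second delay loop, with no target actor or destination shown.
; A hit from the player enables mesh physics and destroys the capsule, with no explicit stop to the move loop.
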(event OnSeePawn(PawnSensing)
  (params (Pawn :type Pawn%20Object%20Reference))
  (Utilities|Casting|CastToBP_FirstPersonCharacter Pawn)
  (Variables|Default|SetChasing true) ; go back to patrolling
  (AI|AIMoveTo self "0, 0, 0" 0 1e+02 false :!label _label
    (:then
      (Utilities|FlowControl|Delay 0.2)
      (goto _label))))

(event Collision|EventHit
  (params (MyComp :type Primitive%20Component%20Object%20Reference) (Other :type Actor%20Object%20Reference) (OtherComp :type Primitive%20Component%20Object%20Reference) (bSelfMoved :type Boolean) (HitLocation :type Vector :default "0, 0, 0") (HitNormal :type Vector :default "0, 0, 0") (NormalImpulse :type Vector :default "0, 0, 0") (Hit :type Hit%20Result%20Structure%20%28by%20ref%29))
  (Utilities|Casting|CastToBP_FirstPersonCharacter Other)
  (Physics|SetSimulatePhysics (Variables|Character|GetMesh) true)
  (Components|DestroyComponent (Variables|Collision|GetCapsuleComponent)))

(fn ConstructionScript)