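; BP_PatrolRoute is a patrol route for AI that supplies successive world-space locations from the points of a spline.
; GetPatrolPointLocation first calls IncPatrolPointIndex, then returns the location of the spline point at the new index.
; IncPatrolPointIndex steps the index by Direction, flipping it once the index exceeds the point count or falls to zero or below, giving back-and-forth traversal.
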(event Custom|Inc%20Patrol%20Point%20Index
  (Variables|Default|SetPatrol%20Index (+ (Variables|Default|GetPatrol%20Index) (Variables|Default|GetDirection)))
  (if (> (Variables|Default|GetPatrol%20Index) (Spline|GetNumberOfSplinePoints (Variables|Default|GetSpline)))
    ;[1 1 1] Flip Direction
    (Variables|Default|SetDirection -1)
    (else
      ;[1 1 1] If at beginning, start over
      (if (<= (Variables|Default|GetPatrol%20Index) 0)
        (Variables|Default|SetDirection 1)))))

(fn ConstructionScript)

(fn GetPatrolPointLocation
  (CallFunction|IncPatrolPointIndex)
  (return (Spline|GetLocationatSplinePoint (Variables|Default|GetSpline) (Variables|Default|GetPatrol%20Index) "World")))