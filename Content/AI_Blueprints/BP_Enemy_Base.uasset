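; Base enemy Blueprint that serves as the pawn side of an AIC_Enemy_Base-controlled AI.
; After a short BeginPlay delay, it passes its start state and the player as attack target to that controller.
; It exposes speed presets and an Attack event that plays a montage, then broadcasts OnAttackEnd on completion or interruption.
; SetState and both fire events are empty stubs, with hand-fire attach and destroy logic left disconnected.
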(event Custom|Attack
  (Animation|Montage|PlayMontage (Variables|Character|GetMesh) 0
    (:OnCompleted
      _)
    (:OnInterrupted
      _))
  (Default|CallOnAttackEnd))

(event Custom|Spawn%20Fire)

(event Custom|Extinguish%20Fire)

(event Custom|Set%20Movement%20Speed
  (params (Speed :type E_MovementSpeed%20Enum :default "NewEnumerator0"))
  (Variables|/Script/Engine.CharacterMovementComponent|SetMaxWalkSpeed (Variables|Character|GetCharacterMovement) (Utilities|Select :Index Speed :NewEnumerator0 0.0 :NewEnumerator1 3e+02 :NewEnumerator2 5e+02 :NewEnumerator3 7.5e+02)))

(event EventBeginPlay
  (Utilities|FlowControl|Delay 0.3)
  (bind _asaic_enemy_base (Utilities|Casting|CastToAIC_Enemy_Base (AI|GetAIController self)))
  (Default|SetState _asaic_enemy_base (Variables|Default|GetStartState) (Game|GetPlayerCharacter 0) "0, 0, 0"))

(fn ConstructionScript)

(fn SetState
  (params (New%20State :type E_AIState%20Enum :default "NewEnumerator0") (Attack%20Target :type Actor%20Object%20Reference)))