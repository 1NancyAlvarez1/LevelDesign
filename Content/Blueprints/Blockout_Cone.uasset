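; Blockout cone actor for level prototyping, built entirely in the construction script with no active runtime logic.
; It passes radius and height through a rounding helper using RoundSize, then adds a static mesh component scaled from centimeters to those dimensions.
; ConeQuality selects the mesh from an array of cone variants, and a shared blockout helper then sets the material.
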(event EventBeginPlay)

(event Collision|EventActorBeginOverlap
  (params (OtherActor :type Actor%20Object%20Reference)))

(event EventTick
  (params (DeltaSeconds :type Float%20%28single-precision%29)))

(fn ConstructionScript
  (CallFunction|BlockoutRoundFloat (Variables|BlockoutTools|BlockoutCone|GetbRoundSize) (Variables|BlockoutTools|BlockoutCone|GetConeRadius))
  (CallFunction|BlockoutRoundFloat (Variables|BlockoutTools|BlockoutCone|GetbRoundSize) (Variables|BlockoutTools|BlockoutCone|GetConeHeight))
  (CallFunction|AddBlockoutCone)
  (Class|BlockoutToolsParent|BlockoutSetMaterial))

(fn AddBlockoutCone
  (bind _returnvalue (/ 1.0 1e+02))
  (bind _coneradius (Variables|BlockoutTools|BlockoutCone|GetConeRadius))
  (bind _returnvalue_2 (* _coneradius 2.0))
  (bind _returnvalue_3 (* _returnvalue_2 _returnvalue))
  (bind _returnvalue_4 (AddComponent|AddStaticMeshComponent false (Math|Transform|MakeTransform "0, 0, 0" "0, 0, 0" (Math|Vector|MakeVector _returnvalue_3 _returnvalue_3 (* (Variables|BlockoutTools|BlockoutCone|GetConeHeight) (/ 1.0 1e+02))))))
  (Components|StaticMesh|SetStaticMesh _returnvalue_4 (Utilities|Array|Get(acopy) (Variables|BlockoutTools|BlockoutCone|GetBlockoutConeMeshes) (Variables|BlockoutTools|BlockoutCone|GetConeQuality))))