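; Blockout corner ramp actor, a resizable greybox piece built entirely in the construction script.
; It rounds CornerRampSize by RoundSize, adds a static mesh component using the corner ramp mesh, then applies the blockout material.
; The mesh is scaled by the size divided by 100, so dimensions are entered in Unreal units rather than as scale factors.
; The event graph holds no active logic.
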(event EventBeginPlay)

(event Collision|EventActorBeginOverlap
  (params (OtherActor :type Actor%20Object%20Reference)))

(event EventTick
  (params (DeltaSeconds :type Float%20%28single-precision%29)))

(fn ConstructionScript
  (CallFunction|BlockoutRoundVector (Variables|BlockoutTools|BlockoutCornerRamp|GetbRoundSize) (Variables|BlockoutTools|BlockoutCornerRamp|GetCornerRampSize))
  (CallFunction|AddBlockoutCornerRamp)
  (Class|BlockoutToolsParent|BlockoutSetMaterial))

(fn AddBlockoutCornerRamp
  (bind _returnvalue (AddComponent|AddStaticMeshComponent false (Math|Transform|MakeTransform "0, 0, 0" "0, 0, 0" (* (Variables|BlockoutTools|BlockoutCornerRamp|GetCornerRampSize) (/ 1.0 1e+02)))))
  (Components|StaticMesh|SetStaticMesh _returnvalue (Variables|BlockoutTools|BlockoutCornerRamp|GetBlockoutCornerRampMesh)))