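; Blockout actor that builds a straight staircase in the construction script from a manually set step count and step dimensions.
; It rounds the dimensions and spacings via BlockoutRoundFloat, adds one scaled static mesh per step, then applies the blockout material.
; StairsType selects box steps, sloped steps, or solid steps that grow taller from the base, with spacing applied only to the first two.
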(event EventBeginPlay)

(event Collision|EventActorBeginOverlap
  (params (OtherActor :type Actor%20Object%20Reference)))

(event EventTick
  (params (DeltaSeconds :type Float%20%28single-precision%29)))

(fn ConstructionScript
  (CallFunction|BlockoutRoundFloat (Variables|BlockoutTools|BlockoutStairsLinearManual|GetbRoundSize) (Variables|BlockoutTools|BlockoutStairsLinearManual|GetStepWidth))
  (CallFunction|BlockoutRoundFloat (Variables|BlockoutTools|BlockoutStairsLinearManual|GetbRoundSize) (Variables|BlockoutTools|BlockoutStairsLinearManual|GetStepDepth))
  (CallFunction|BlockoutRoundFloat (Variables|BlockoutTools|BlockoutStairsLinearManual|GetbRoundSize) (Variables|BlockoutTools|BlockoutStairsLinearManual|GetStepHeight))
  (CallFunction|BlockoutRoundFloat (Variables|BlockoutTools|BlockoutStairsLinearManual|GetbRoundSize) (Variables|BlockoutTools|BlockoutStairsLinearManual|GetStepDepthSpacing))
  (CallFunction|BlockoutRoundFloat (Variables|BlockoutTools|BlockoutStairsLinearManual|GetbRoundSize) (Variables|BlockoutTools|BlockoutStairsLinearManual|GetStepHeightSpacing))
  (CallFunction|AddBlockoutStairsLinearManual)
  (Class|BlockoutToolsParent|BlockoutSetMaterial))

(fn AddBlockoutStairsLinearManual
  (bind _stepheight (Variables|BlockoutTools|BlockoutStairsLinearManual|GetStepHeight))
  (for _index (range 0 (- (Variables|BlockoutTools|BlockoutStairsLinearManual|GetNumberOfSteps) 1))
    (bind _returnvalue (AddComponent|AddStaticMeshComponent false (Math|Transform|MakeTransform (Math|Vector|MakeVector 0.0 (Utilities|Select :Index (Variables|BlockoutTools|BlockoutStairsLinearManual|GetStairsType) :Option%200 (+ (* _index (Variables|BlockoutTools|BlockoutStairsLinearManual|GetStepDepth)) (* _index (Variables|BlockoutTools|BlockoutStairsLinearManual|GetStepDepthSpacing))) :Option%201 (+ (* _index (Variables|BlockoutTools|BlockoutStairsLinearManual|GetStepDepth)) (* _index (Variables|BlockoutTools|BlockoutStairsLinearManual|GetStepDepthSpacing))) :Option%202 (* _index (Variables|BlockoutTools|BlockoutStairsLinearManual|GetStepDepth))) (Utilities|Select :Index (Variables|BlockoutTools|BlockoutStairsLinearManual|GetStairsType) :Option%200 (+ (* _index (Variables|BlockoutTools|BlockoutStairsLinearManual|GetStepHeight)) (* _index (Variables|BlockoutTools|BlockoutStairsLinearManual|GetStepHeightSpacing))) :Option%201 (+ (* _index (Variables|BlockoutTools|BlockoutStairsLinearManual|GetStepHeight)) (* _index (Variables|BlockoutTools|BlockoutStairsLinearManual|GetStepHeightSpacing))) :Option%202 0.0)) "0, 0, 0" (* (/ "1.000000,1.000000,1.000000" 1e+02) (Math|Vector|MakeVector (Variables|BlockoutTools|BlockoutStairsLinearManual|GetStepWidth) (Variables|BlockoutTools|BlockoutStairsLinearManual|GetStepDepth) (Utilities|Select :Index (Variables|BlockoutTools|BlockoutStairsLinearManual|GetStairsType) :Option%200 _stepheight :Option%201 _stepheight :Option%202 (* (+ _index 1) (Variables|BlockoutTools|BlockoutStairsLinearManual|GetStepHeight))))))))
    (Components|StaticMesh|SetStaticMesh _returnvalue (Utilities|Select :Index (Variables|BlockoutTools|BlockoutStairsLinearManual|GetStairsType) :Option%200 "/BlockoutToolsPlugin/Meshes/SM_Blockout_Step_Box.SM_Blockout_Step_Box" :Option%201 "/BlockoutToolsPlugin/Meshes/SM_Blockout_Step_Sloped_Linear.SM_Blockout_Step_Sloped_Linear" :Option%202 "/BlockoutToolsPlugin/Meshes/SM_Blockout_Step_Box.SM_Blockout_Step_Box"))))