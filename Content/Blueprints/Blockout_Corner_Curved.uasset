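; Blockout actor for a curved corner piece, used to grey-box level geometry and rebuilt in the construction script.
; It rounds radius and height to the round size, then adds a static mesh component scaled from those values in centimetres.
; The mesh comes from an inner or outer array, indexed by a quality setting.
; A shared blockout function then applies the material.
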(event EventBeginPlay)

(event Collision|EventActorBeginOverlap
  (params (OtherActor :type Actor%20Object%20Reference)))

(event EventTick
  (params (DeltaSeconds :type Float%20%28single-precision%29)))

(fn ConstructionScript
  (CallFunction|BlockoutRoundFloat (Variables|BlockoutTools|BlockoutCornerCurved|GetbRoundSize) (Variables|BlockoutTools|BlockoutCornerCurved|GetCornerCurvedRadius))
  (CallFunction|BlockoutRoundFloat (Variables|BlockoutTools|BlockoutCornerCurved|GetbRoundSize) (Variables|BlockoutTools|BlockoutCornerCurved|GetCornerCurvedHeight))
  (CallFunction|AddBlockoutCornerCurved)
  (Class|BlockoutToolsParent|BlockoutSetMaterial))

(fn AddBlockoutCornerCurved
  (bind _returnvalue (/ 1.0 1e+02))
  (bind _cornercurvedradius (Variables|BlockoutTools|BlockoutCornerCurved|GetCornerCurvedRadius))
  (bind _returnvalue_2 (* _cornercurvedradius _returnvalue))
  (bind _returnvalue_3 (AddComponent|AddStaticMeshComponent false (Math|Transform|MakeTransform "0, 0, 0" "0, 0, 0" (Math|Vector|MakeVector _returnvalue_2 _returnvalue_2 (* (Variables|BlockoutTools|BlockoutCornerCurved|GetCornerCurvedHeight) (/ 1.0 1e+02))))))
  (Components|StaticMesh|SetStaticMesh _returnvalue_3 (select (Variables|BlockoutTools|BlockoutCornerCurved|GetbIsInner) (Utilities|Array|Get(acopy) (Variables|BlockoutTools|BlockoutCornerCurved|GetBlockoutCornerMeshesInner) (Variables|BlockoutTools|BlockoutCornerCurved|GetCornerCurvedQuality)) (Utilities|Array|Get(acopy) (Variables|BlockoutTools|BlockoutCornerCurved|GetBlockoutCornerMeshesOuter) (Variables|BlockoutTools|BlockoutCornerCurved|GetCornerCurvedQuality)))))