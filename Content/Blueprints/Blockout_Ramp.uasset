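; Blockout ramp actor for greyboxing levels, sized through a RampSize vector.
; The construction script passes RampSize and RoundSize to a rounding helper, adds the ramp mesh, then applies the blockout material.
; The mesh is a dynamically added static mesh component scaled by RampSize / 100, so size values map to units on a presumably 100-unit mesh.
; The event graph holds no active logic.
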(event EventBeginPlay)

(event Collision|EventActorBeginOverlap
  (params (OtherActor :type Actor%20Object%20Reference)))

(event EventTick
  (params (DeltaSeconds :type Float%20%28single-precision%29)))

(fn ConstructionScript
  (CallFunction|BlockoutRoundVector (Variables|BlockoutTools|BlockoutRamp|GetbRoundSize) (Variables|BlockoutTools|BlockoutRamp|GetRampSize))
  (CallFunction|AddBlockoutRamp)
  (Class|BlockoutToolsParent|BlockoutSetMaterial))

(fn AddBlockoutRamp
  (bind _returnvalue (AddComponent|AddStaticMeshComponent false (Math|Transform|MakeTransform "0, 0, 0" "0, 0, 0" (* (Variables|BlockoutTools|BlockoutRamp|GetRampSize) (/ 1.0 1e+02)))))
  (Components|StaticMesh|SetStaticMesh _returnvalue (Variables|BlockoutTools|BlockoutRamp|GetBlockoutRampMesh)))