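; Blockout railing actor for level prototyping that builds a straight, optionally sloped railing procedurally in the construction script.
; It rounds section length and skew elevation, then places a pole mesh at each section boundary, with an optional end pole.
; Spline meshes, open or closed by railing type, bridge the poles, with height interpolated linearly along the run.
; A blockout material pass finishes the build, and no runtime logic runs.
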(event EventBeginPlay)

(event Collision|EventActorBeginOverlap
  (params (OtherActor :type Actor%20Object%20Reference)))

(event EventTick
  (params (DeltaSeconds :type Float%20%28single-precision%29)))

(fn ConstructionScript
  (CallFunction|BlockoutRoundFloat (Variables|BlockoutTools|BlockoutRailing|GetbRoundSize) (Variables|BlockoutTools|BlockoutRailing|GetSectionLenght))
  (CallFunction|BlockoutRoundFloat (Variables|BlockoutTools|BlockoutRailing|GetbRoundSize) (Variables|BlockoutTools|BlockoutRailing|GetSkewElevation))
  (CallFunction|AddBlockoutRailing)
  (Class|BlockoutToolsParent|BlockoutSetMaterial))

(fn AddBlockoutRailing
  (for _index (range 0 (select (Variables|BlockoutTools|BlockoutRailing|GetbHasEndPole) (Variables|BlockoutTools|BlockoutRailing|GetRailingSections) (- (Variables|BlockoutTools|BlockoutRailing|GetRailingSections) 1)))
    (bind _returnvalue (AddComponent|AddStaticMeshComponent false (Math|Transform|MakeTransform (Math|Vector|MakeVector (* _index (Variables|BlockoutTools|BlockoutRailing|GetSectionLenght)) 0.0 (CallFunction|GetCurrentHeight _index (Variables|BlockoutTools|BlockoutRailing|GetRailingSections) (Variables|BlockoutTools|BlockoutRailing|GetSkewElevation))))))
    (Components|StaticMesh|SetStaticMesh _returnvalue (Variables|BlockoutTools|BlockoutRailing|GetBlockoutRailingPoleMesh))
    (if (<= (+ _index 1) (Variables|BlockoutTools|BlockoutRailing|GetRailingSections))
      (bind _returnvalue_2 (AddComponent|AddSplineMeshComponent false))
      (Components|StaticMesh|SetStaticMesh _returnvalue_2 (Utilities|Select :Index (Variables|BlockoutTools|BlockoutRailing|GetRailingType) :NewEnumerator0 "/BlockoutToolsPlugin/Meshes/SM_Blockout_Railing_Open.SM_Blockout_Railing_Open" :NewEnumerator1 "/BlockoutToolsPlugin/Meshes/SM_Blockout_Railing_Closed.SM_Blockout_Railing_Closed"))
      (SplineMesh|SetStartandEnd _returnvalue_2 (Math|Vector|MakeVector (* _index (Variables|BlockoutTools|BlockoutRailing|GetSectionLenght)) 0.0 (CallFunction|GetCurrentHeight _index (Variables|BlockoutTools|BlockoutRailing|GetRailingSections) (Variables|BlockoutTools|BlockoutRailing|GetSkewElevation))) "100.000000, 0, 0" (Math|Vector|MakeVector (* (+ _index 1) (Variables|BlockoutTools|BlockoutRailing|GetSectionLenght)) 0.0 (CallFunction|GetCurrentHeight (+ _index 1) (Variables|BlockoutTools|BlockoutRailing|GetRailingSections) (Variables|BlockoutTools|BlockoutRailing|GetSkewElevation))) "100.000000, 0, 0" true :!class /Script/Engine.SplineMeshComponent))))

(fn GetCurrentHeight
  (params (Index :type Integer) (RailingSections :type Integer) (SkewHeight :type Float%20%28double-precision%29))
  (return (* (/ (Math|Conversions|ToFloat(Integer) Index) (Math|Conversions|ToFloat(Integer) RailingSections)) SkewHeight)))