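; BP_EntrancePuzzle is a trigger volume that shows two timed dialog widgets when the first-person character enters its Box.
; The overlap passes a character cast and a DoOnce, so the sequence runs only once.
; It displays W_Entrance, then W_CheckClassrooms, each removed from the viewport after a short delay.
; Despite the name, the Blueprint contains no puzzle logic, only this message sequence.
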(event OnComponentBeginOverlap(Box)
  (params (OverlappedComponent :type Primitive%20Component%20Object%20Reference) (OtherActor :type Actor%20Object%20Reference) (OtherComp :type Primitive%20Component%20Object%20Reference) (OtherBodyIndex :type Integer) (bFromSweep :type Boolean) (SweepResult :type Hit%20Result%20Structure%20%28by%20ref%29))
  (Utilities|Casting|CastToBP_FirstPersonCharacter OtherActor)
  (Utilities|FlowControl|DoOnce false
    (:Completed
      (bind _returnvalue (UserInterface|CreateWidget "/Game/Widgets/W_Entrance.W_Entrance_C"))
      (bind _output_get (Variables|Default|SetDialog _returnvalue))
      (UserInterface|Viewport|AddtoViewport _output_get 0)
      (Utilities|FlowControl|Delay 3.0)
      (Widget|RemovefromParent _returnvalue)
      (bind _returnvalue_2 (UserInterface|CreateWidget "/Game/Widgets/W_CheckClassrooms.W_CheckClassrooms_C"))
      (bind _output_get_2 (Variables|Default|SetDialog2 _returnvalue_2))
      (UserInterface|Viewport|AddtoViewport _output_get_2 0)
      (Utilities|FlowControl|Delay 3.0)
      (Widget|RemovefromParent _returnvalue_2))))

(event EventBeginPlay)

(event Collision|EventActorBeginOverlap
  (params (OtherActor :type Actor%20Object%20Reference)))

(event EventTick
  (params (DeltaSeconds :type Float%20%28single-precision%29)))

(fn ConstructionScript)