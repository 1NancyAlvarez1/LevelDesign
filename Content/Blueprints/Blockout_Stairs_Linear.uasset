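; Blockout actor that procedurally builds a straight staircase for level prototyping in its construction script.
; It rounds the stair size, divides it by the step count, then adds one scaled static mesh component per step along Y and applies the blockout material.
; StairsType selects stacked box steps, sloped-mesh steps, or solid box steps that grow in height from the base.
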(event EventBeginPlay)

(event Collision|EventActorBeginOverlap
  (params (OtherActor :type Actor%20Object%20Reference)))

(event EventTick
  (params (DeltaSeconds :type Float%20%28single-precision%29)))

(fn ConstructionScript
  (CallFunction|BlockoutRoundVector (Variables|BlockoutTools|BlockoutStairsLinear|GetbRoundSize) (Variables|BlockoutTools|BlockoutStairsLinear|GetStairsSize))
  (CallFunction|SetupStepSizes)
  (CallFunction|AddBlockoutStairsLinear)
  (Class|BlockoutToolsParent|BlockoutSetMaterial))

(fn AddBlockoutStairsLinear
  (bind _stepheight (Variables|BlockoutTools|BlockoutStairsLinear|GetStepHeight))
  (for _index (range 0 (- (Variables|BlockoutTools|BlockoutStairsLinear|GetNumberOfSteps) 1))
    (bind _returnvalue (AddComponent|AddStaticMeshComponent false (Math|Transform|MakeTransform (Math|Vector|MakeVector 0.0 (* _index (Variables|BlockoutTools|BlockoutStairsLinear|GetStepDepth)) (Utilities|Select :Index (Variables|BlockoutTools|BlockoutStairsLinear|GetStairsType) :Option%200 (* _index (Variables|BlockoutTools|BlockoutStairsLinear|GetStepHeight)) :Option%201 (* _index (Variables|BlockoutTools|BlockoutStairsLinear|GetStepHeight)) :Option%202 0.0)) "0, 0, 0" (* (/ "1.000000,1.000000,1.000000" 1e+02) (Math|Vector|MakeVector (Variables|BlockoutTools|BlockoutStairsLinear|GetStepWidth) (Variables|BlockoutTools|BlockoutStairsLinear|GetStepDepth) (Utilities|Select :Index (Variables|BlockoutTools|BlockoutStairsLinear|GetStairsType) :Option%200 _stepheight :Option%201 _stepheight :Option%202 (* (+ _index 1) (Variables|BlockoutTools|BlockoutStairsLinear|GetStepHeight))))))))
    (Components|StaticMesh|SetStaticMesh _returnvalue (Utilities|Select :Index (Variables|BlockoutTools|BlockoutStairsLinear|GetStairsType) :Option%200 "/BlockoutToolsPlugin/Meshes/SM_Blockout_Step_Box.SM_Blockout_Step_Box" :Option%201 "/BlockoutToolsPlugin/Meshes/SM_Blockout_Step_Sloped_Linear.SM_Blockout_Step_Sloped_Linear" :Option%202 "/BlockoutToolsPlugin/Meshes/SM_Blockout_Step_Box.SM_Blockout_Step_Box"))))

(fn SetupStepSizes
  (Variables|BlockoutTools|BlockoutStairsLinear|SetStepWidth (.X (Math|Vector|BreakVector (Variables|BlockoutTools|BlockoutStairsLinear|GetStairsSize))))
  (Variables|BlockoutTools|BlockoutStairsLinear|SetStepDepth (/ (.Y (Math|Vector|BreakVector (Variables|BlockoutTools|BlockoutStairsLinear|GetStairsSize))) (Math|Conversions|ToFloat(Integer) (Variables|BlockoutTools|BlockoutStairsLinear|GetNumberOfSteps))))
  (Variables|BlockoutTools|BlockoutStairsLinear|SetStepHeight (/ (.Z (Math|Vector|BreakVector (Variables|BlockoutTools|BlockoutStairsLinear|GetStairsSize))) (Math|Conversions|ToFloat(Integer) (Variables|BlockoutTools|BlockoutStairsLinear|GetNumberOfSteps)))))