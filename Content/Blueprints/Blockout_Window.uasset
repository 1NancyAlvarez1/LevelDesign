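; Blockout window actor that builds a resizable, four-piece window casing for level blockout.
; The construction script passes window size and top, side and bottom thicknesses through rounding helpers by RoundSize, builds the casing, then calls BlockoutSetMaterial.
; AddBlockoutWindow spawns left, top, right and bottom static mesh components from one shared mesh, scaled and offset to leave an open center.
; The event graph has no active logic.
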(event EventBeginPlay)

(event Collision|EventActorBeginOverlap
  (params (OtherActor :type Actor%20Object%20Reference)))

(event EventTick
  (params (DeltaSeconds :type Float%20%28single-precision%29)))

(fn ConstructionScript
  (CallFunction|BlockoutRoundVector (Variables|BlockoutTools|BlockoutWindow|GetbRoundSize) (Variables|BlockoutTools|BlockoutWindow|GetWindowSize))
  (CallFunction|BlockoutRoundFloat (Variables|BlockoutTools|BlockoutWindow|GetbRoundSize) (Variables|BlockoutTools|BlockoutWindow|GetTopThickness))
  (CallFunction|BlockoutRoundFloat (Variables|BlockoutTools|BlockoutWindow|GetbRoundSize) (Variables|BlockoutTools|BlockoutWindow|GetSideThickness))
  (CallFunction|BlockoutRoundFloat (Variables|BlockoutTools|BlockoutWindow|GetbRoundSize) (Variables|BlockoutTools|BlockoutWindow|GetBottomThickness))
  (CallFunction|AddBlockoutWindow)
  (Class|BlockoutToolsParent|BlockoutSetMaterial))

(fn AddBlockoutWindow
  (bind _windowsize (Variables|BlockoutTools|BlockoutWindow|GetWindowSize))
  (bind _windowsize_2 (Variables|BlockoutTools|BlockoutWindow|GetWindowSize))
  (bind _windowsize_3 (Variables|BlockoutTools|BlockoutWindow|GetWindowSize))
  (bind _windowsize_4 (Variables|BlockoutTools|BlockoutWindow|GetWindowSize))
  (bind (_x _y _z) (Math|Vector|BreakVector _windowsize_4))
  (bind (_x_2 _y_2 _z_2) (Math|Vector|BreakVector _windowsize_2))
  (bind (_x_3 _y_3) (Math|Vector|BreakVector _windowsize_3))
  (bind (_x_4 _y_4) (Math|Vector|BreakVector _windowsize))
  (bind _returnvalue (AddComponent|AddStaticMeshComponent false (Math|Transform|MakeTransform "0, 0, 0" "0, 0, 0" (* (Math|Vector|MakeVector _x (Variables|BlockoutTools|BlockoutWindow|GetSideThickness) _z) (/ 1.0 1e+02))))) ; Casing Left
  (Components|StaticMesh|SetStaticMesh _returnvalue (Variables|BlockoutTools|BlockoutWindow|GetBlockoutWindowMesh))
  (bind _returnvalue_2 (AddComponent|AddStaticMeshComponent false (Math|Transform|MakeTransform (Math|Vector|MakeVector 0.0 (Variables|BlockoutTools|BlockoutWindow|GetSideThickness) (- (.Z (Math|Vector|BreakVector (Variables|BlockoutTools|BlockoutWindow|GetWindowSize))) (Variables|BlockoutTools|BlockoutWindow|GetTopThickness))) "0, 0, 0" (* (Math|Vector|MakeVector _x_4 (- _y_4 (* (Variables|BlockoutTools|BlockoutWindow|GetSideThickness) 2.0)) (Variables|BlockoutTools|BlockoutWindow|GetTopThickness)) (/ 1.0 1e+02))))) ; Casing Top
  (Components|StaticMesh|SetStaticMesh _returnvalue_2 (Variables|BlockoutTools|BlockoutWindow|GetBlockoutWindowMesh))
  (bind _returnvalue_3 (AddComponent|AddStaticMeshComponent false (Math|Transform|MakeTransform (Math|Vector|MakeVector 0.0 (- (.Y (Math|Vector|BreakVector (Variables|BlockoutTools|BlockoutWindow|GetWindowSize))) (Variables|BlockoutTools|BlockoutWindow|GetSideThickness)) 0.0) "0, 0, 0" (* (Math|Vector|MakeVector _x_2 (Variables|BlockoutTools|BlockoutWindow|GetSideThickness) _z_2) (/ 1.0 1e+02))))) ; Casing Right
  (Components|StaticMesh|SetStaticMesh _returnvalue_3 (Variables|BlockoutTools|BlockoutWindow|GetBlockoutWindowMesh))
  (bind _returnvalue_4 (AddComponent|AddStaticMeshComponent false (Math|Transform|MakeTransform (Math|Vector|MakeVector 0.0 (Variables|BlockoutTools|BlockoutWindow|GetSideThickness) 0.0) "0, 0, 0" (* (Math|Vector|MakeVector _x_3 (- _y_3 (* (Variables|BlockoutTools|BlockoutWindow|GetSideThickness) 2.0)) (Variables|BlockoutTools|BlockoutWindow|GetBottomThickness)) (/ 1.0 1e+02))))) ; Casing Bottom
  (Components|StaticMesh|SetStaticMesh _returnvalue_4 (Variables|BlockoutTools|BlockoutWindow|GetBlockoutWindowMesh)))