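; Utility functions for blockout tools that handle optional size rounding and material setup on blockout meshes.
; The rounding helpers snap floats, vectors and 2D vectors to whole numbers when RoundSize is set, either returning all three at once or writing back to a by-ref input.
; The material helper creates a dynamic instance of the blockout material, sets grid, color and top-color parameters, and assigns it to the mesh's first slot.
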(fn BlockoutRoundVariablesD
  (params (RoundSize :type Boolean) (InFloat :type Float%20%28double-precision%29) (InVector :type Vector) (InVector2D :type Vector%202D%20Structure))
  (bind (_x _y) (Math|Vector2D|BreakVector2D InVector2D))
  (bind (_x_2 _y_2 _z) (Math|Vector|BreakVector InVector))
  (return (select RoundSize (Math|Conversions|ToFloat(Integer) (Math|Float|Round InFloat)) InFloat) (select RoundSize (Math|Vector|MakeVector (Math|Conversions|ToFloat(Integer) (Math|Float|Round _x_2)) (Math|Conversions|ToFloat(Integer) (Math|Float|Round _y_2)) (Math|Conversions|ToFloat(Integer) (Math|Float|Round _z))) InVector) (select RoundSize (Math|Vector2D|MakeVector2D (Math|Conversions|ToFloat(Integer) (Math|Float|Round _x)) (Math|Conversions|ToFloat(Integer) (Math|Float|Round _y))) InVector2D)))

(fn BlockoutSetMaterialD
  (params (StaticMesh :type Mesh%20Component%20Object%20Reference) (BlockoutMaterial :type Material%20Interface%20Object%20Reference) (UseGrid :type Boolean) (Color :type Linear%20Color%20Structure) (UseTopColor :type Boolean) (TopColor :type Linear%20Color%20Structure))
  (bind _returnvalue (Rendering|Material|CreateDynamicMaterialInstance 0 BlockoutMaterial "None" :!class /Script/Engine.KismetMaterialLibrary))
  (Rendering|Material|SetScalarParameterValue _returnvalue "GridAlpha" (select UseGrid 1.0 0.0) :!class /Script/Engine.MaterialInstanceDynamic)
  (Rendering|Material|SetVectorParameterValue _returnvalue "Color" Color :!class /Script/Engine.MaterialInstanceDynamic)
  (Rendering|Material|SetScalarParameterValue _returnvalue "TopColorAlpha" (select UseTopColor 1.0 0.0) :!class /Script/Engine.MaterialInstanceDynamic)
  (Rendering|Material|SetVectorParameterValue _returnvalue "TopColor" TopColor :!class /Script/Engine.MaterialInstanceDynamic)
  (Rendering|Material|SetMaterial StaticMesh 0 _returnvalue))

(fn BlockoutRoundFloat
  (params (RoundSize :type Boolean) (Float :type Float%20%28double-precision%29%20%28by%20ref%29))
  (|SetBy-RefVar Float (select RoundSize (Math|Conversions|ToFloat(Integer) (Math|Float|Round Float)) Float))
  (return))

(fn BlockoutRoundVector
  (params (RoundSize :type Boolean) (Vector :type Vector%20%28by%20ref%29))
  (bind (_x _y _z) (Math|Vector|BreakVector Vector))
  (|SetBy-RefVar Vector (select RoundSize (Math|Vector|MakeVector (Math|Conversions|ToFloat(Integer) (Math|Float|Round _x)) (Math|Conversions|ToFloat(Integer) (Math|Float|Round _y)) (Math|Conversions|ToFloat(Integer) (Math|Float|Round _z))) Vector))
  (return))

(fn BlockoutRoundVector2D
  (params (RoundSize :type Boolean) (Vector :type Vector%202D%20Structure%20%28by%20ref%29))
  (|SetBy-RefVar Vector (select RoundSize (Class|KismetMathLibrary|ToRounded2D Vector) Vector))
  (return))