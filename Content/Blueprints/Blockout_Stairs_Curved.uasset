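; Blockout actor that procedurally builds a curved staircase in the construction script for level prototyping.
; It rounds angle, height, inner radius and width, derives per-step height and arc-based inner and outer widths, then adds one spline mesh per step, rotated around the origin.
; Tapering start and end scales form wedge steps; StairsType selects box, sloped or solid floor-reaching steps, with optional counter-clockwise winding.
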(event EventBeginPlay)

(event Collision|EventActorBeginOverlap
  (params (OtherActor :type Actor%20Object%20Reference)))

(event EventTick
  (params (DeltaSeconds :type Float%20%28single-precision%29)))

(fn ConstructionScript
  (CallFunction|BlockoutRoundFloat (Variables|BlockoutTools|BlockoutStairsCurved|GetbRoundSize) (Variables|BlockoutTools|BlockoutStairsCurved|GetStairsAngle))
  (CallFunction|BlockoutRoundFloat (Variables|BlockoutTools|BlockoutStairsCurved|GetbRoundSize) (Variables|BlockoutTools|BlockoutStairsCurved|GetStairsHeight))
  (CallFunction|BlockoutRoundFloat (Variables|BlockoutTools|BlockoutStairsCurved|GetbRoundSize) (Variables|BlockoutTools|BlockoutStairsCurved|GetInnerRadius))
  (CallFunction|BlockoutRoundFloat (Variables|BlockoutTools|BlockoutStairsCurved|GetbRoundSize) (Variables|BlockoutTools|BlockoutStairsCurved|GetStepWidth))
  (CallFunction|SetupStepSizes)
  (CallFunction|AddBlockoutStairsCurved)
  (Class|BlockoutToolsParent|BlockoutSetMaterial))

(fn AddBlockoutStairsCurved
  (bind _bcounterclockwise (Variables|BlockoutTools|BlockoutStairsCurved|GetbCounterClockwise))
  (bind _stairsangle (Variables|BlockoutTools|BlockoutStairsCurved|GetStairsAngle))
  (bind _endsize (Variables|BlockoutTools|BlockoutStairsCurved|GetEndSize))
  (bind _numberofsteps (Variables|BlockoutTools|BlockoutStairsCurved|GetNumberOfSteps))
  (bind _stairsangle_2 (Variables|BlockoutTools|BlockoutStairsCurved|GetStairsAngle))
  (bind _startsize (Variables|BlockoutTools|BlockoutStairsCurved|GetStartSize))
  (bind _returnvalue (Math|Conversions|ToFloat(Integer) _numberofsteps))
  (bind _returnvalue_2 (* _stairsangle -1.0))
  (bind _returnvalue_3 (select _bcounterclockwise _returnvalue_2 _stairsangle_2))
  (bind _returnvalue_4 (/ _returnvalue_3 _returnvalue))
  (for _index (range 0 (- (Variables|BlockoutTools|BlockoutStairsCurved|GetNumberOfSteps) 1))
    (bind _returnvalue_5 (AddComponent|AddSplineMeshComponent false (Math|Transform|MakeTransform "0, 0, 0" (Math|Rotator|MakeRotator 0.0 0.0 (+ (/ _returnvalue_4 2.0) (* _index _returnvalue_4))))))
    (Components|StaticMesh|SetStaticMesh _returnvalue_5 (Utilities|Select :Index (Variables|BlockoutTools|BlockoutStairsCurved|GetStairsType) :Option%200 "/BlockoutToolsPlugin/Meshes/SM_Blockout_Step_Box_Centered.SM_Blockout_Step_Box_Centered" :Option%201 "/BlockoutToolsPlugin/Meshes/SM_Blockout_Step_Sloped_Centered.SM_Blockout_Step_Sloped_Centered" :Option%202 "/BlockoutToolsPlugin/Meshes/SM_Blockout_Step_Box_Centered.SM_Blockout_Step_Box_Centered"))
    (SplineMesh|SetStartandEnd _returnvalue_5 (Math|Vector|MakeVector (Variables|BlockoutTools|BlockoutStairsCurved|GetInnerRadius) 0.0 (Utilities|Select :Index (Variables|BlockoutTools|BlockoutStairsCurved|GetStairsType) :Option%200 (* _index (Variables|BlockoutTools|BlockoutStairsCurved|GetStepHeight)) :Option%201 (* _index (Variables|BlockoutTools|BlockoutStairsCurved|GetStepHeight)) :Option%202 0.0)) "100.000000,0.000000, 0" (Math|Vector|MakeVector (Variables|BlockoutTools|BlockoutStairsCurved|GetStepWidthSum) 0.0 (Utilities|Select :Index (Variables|BlockoutTools|BlockoutStairsCurved|GetStairsType) :Option%200 (* _index (Variables|BlockoutTools|BlockoutStairsCurved|GetStepHeight)) :Option%201 (* _index (Variables|BlockoutTools|BlockoutStairsCurved|GetStepHeight)) :Option%202 0.0)) "100.000000,0.000000, 0" true :!class /Script/Engine.SplineMeshComponent)
    (SplineMesh|SetStartScale _returnvalue_5 (Utilities|Select :Index (Variables|BlockoutTools|BlockoutStairsCurved|GetStairsType) :Option%200 _startsize :Option%201 _startsize :Option%202 (Utilities|StepHeightbyIndex (Variables|BlockoutTools|BlockoutStairsCurved|GetStartSize) _index)) true :!class /Script/Engine.SplineMeshComponent)
    (SplineMesh|SetEndScale _returnvalue_5 (Utilities|Select :Index (Variables|BlockoutTools|BlockoutStairsCurved|GetStairsType) :Option%200 _endsize :Option%201 _endsize :Option%202 (Utilities|StepHeightbyIndex (Variables|BlockoutTools|BlockoutStairsCurved|GetEndSize) _index)) true :!class /Script/Engine.SplineMeshComponent)))

(fn SetupStepSizes
  (Variables|BlockoutTools|BlockoutStairsCurved|SetStepHeight (/ (Variables|BlockoutTools|BlockoutStairsCurved|GetStairsHeight) (Math|Conversions|ToFloat(Integer) (Variables|BlockoutTools|BlockoutStairsCurved|GetNumberOfSteps))))
  (Variables|BlockoutTools|BlockoutStairsCurved|SetStartSize (/ (Math|Vector2D|MakeVector2D (Utilities|StepWidthbyRadius (Variables|BlockoutTools|BlockoutStairsCurved|GetInnerRadius)) (Variables|BlockoutTools|BlockoutStairsCurved|GetStepHeight)) 1e+02))
  (Variables|BlockoutTools|BlockoutStairsCurved|SetStepWidthSum (+ (Variables|BlockoutTools|BlockoutStairsCurved|GetInnerRadius) (Variables|BlockoutTools|BlockoutStairsCurved|GetStepWidth)))
  (Variables|BlockoutTools|BlockoutStairsCurved|SetEndSize (/ (Math|Vector2D|MakeVector2D (Utilities|StepWidthbyRadius (Variables|BlockoutTools|BlockoutStairsCurved|GetStepWidthSum)) (Variables|BlockoutTools|BlockoutStairsCurved|GetStepHeight)) 1e+02)))